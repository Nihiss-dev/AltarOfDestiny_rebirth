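; Player controller that creates the player info HUD widget and adds it to the viewport when play begins.
; Pressing K casts the controlled pawn to the player character and fetches its Health stat.
; It then prints that stat's type name on screen, which looks like a debug check of the stat system.
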(event `self.ReceiveBeginPlay`
  (bind _returnvalue (`|CreateWidget` "/Game/GUI/Player/W_PlayerInfo.W_PlayerInfo_C" self self))
  (`/Engine/EditorBlueprintResources/StandardMacros.IsValid` _returnvalue
    (:`Is Valid`
      (`UserWidget.AddToViewport` _returnvalue 0))))

(event `Key|K`
  (params (Key :type "Key Structure"))
  (:`Pressed`
    (bind _asbp_player_character (cast `/Game/GameLogic/Player/BP_PlayerCharacter` (`self.K2_GetPawn`)))
    (bind _returnvalue (`S_BaseCharacter.GetStat` _asbp_player_character "Health"))
    (`/Engine/EditorBlueprintResources/StandardMacros.IsValid` _returnvalue
      (:`Is Valid`
        (`KismetSystemLibrary.PrintString` (`|GetEnumeratorNameAsString` (`S_Stat.m_statType` _returnvalue)))))))

(fn `UserConstructionScript`)